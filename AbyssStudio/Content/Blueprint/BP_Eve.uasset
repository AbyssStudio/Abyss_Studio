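; BP_Eve is a first-person shooter character with movement, jump, a crosshair widget and health shown as text.
; Shooting runs a short line trace from the camera and damages any living BP_Eve it hits.
; Events named for server and client split hit handling from health display and death.
; Death sets a flag that blocks shooting and further hits, then restores health after a delay without repositioning.
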(event `self.ReceiveBeginPlay`
  ;[0 1 0.8927] Viseur
  (bind _returnvalue (`|CreateWidget` "/Game/HUD/HUD_Viseur.HUD_Viseur_C"))
  (bind _output_get (set `self.Scope` _returnvalue))
  (`UserWidget.AddToViewport` _output_get 0))

(event `InputAxis|MoveFront`
  (params (AxisValue :type "Float (single-precision)"))
  ;[1 0.076 0] Déplacement
  ;;[1 0.3699 0.1586] Déplacement
  (`self.AddMovementInput` (`KismetMathLibrary.GetForwardVector` (`self.GetControlRotation`)) AxisValue))

(event `InputAxis|MoveSide`
  (params (AxisValue :type "Float (single-precision)"))
  ;[1 0.076 0] Déplacement
  ;;[1 0.3699 0.1586] Déplacement
  (`self.AddMovementInput` (`KismetMathLibrary.GetRightVector` (`self.GetControlRotation`)) AxisValue))

(event `InputAction|Jump`
  (params (Key :type "Key Structure"))
  ;[1 0.076 0] Déplacement
  (:`Pressed`
    (`self.Jump`))
  (:`Released`
    (`self.StopJumping`)))

(event `InputAxis|Turn`
  (params (AxisValue :type "Float (single-precision)"))
  ;[1 0.076 0] Déplacement
  (`self.AddControllerYawInput` AxisValue))

(event `InputAxis|LookUp`
  (params (AxisValue :type "Float (single-precision)"))
  ;[1 0.076 0] Déplacement
  (`self.AddControllerPitchInput` AxisValue))

(event `InputAction|Shoot`
  (params (Key :type "Key Structure"))
  ;[0 0.1533 1] Tir Serveur
  (:`Pressed`
    (if (not (`self.IsDead`))
      (`self.TirServeur`))))

(event `TirServeur`
  (bind _camera (`self.Camera`))
  (bind _returnvalue (`SceneComponent.K2_GetComponentLocation` _camera))
  ;[0 0.1533 1] Tir Serveur
  (bind _outhit (`KismetSystemLibrary.LineTraceSingle` _returnvalue (+ _returnvalue (* (`SceneComponent.GetForwardVector` _camera) 1000.0)) "TraceTypeQuery1"))
  (bind _asbp_eve (cast `/Game/Blueprint/BP_Eve` (`.HitActor` (`GameplayStatics.BreakHitResult` _outhit))))
  (if (not (`/Game/Blueprint/BP_Eve.IsDead` _asbp_eve))
    (`self.Serveur Touche` _asbp_eve)))

(event `Serveur Touche`
  (params (`Player Touche` :type "/Game/Blueprint/BP_Eve Object Reference"))
  (bind _vie (`/Game/Blueprint/BP_Eve.Vie` `Player Touche`))
  ;[1 0.1882 0.9528] Décrement vie
  ;;[1 1 1] serveur touche
  (if (< _vie 0)
    (set `/Game/Blueprint/BP_Eve.IsDead` true `Player Touche`)
    (`self.ClientMort` `Player Touche`)
    (else
      (set `/Game/Blueprint/BP_Eve.Vie` (- _vie 10) `Player Touche`)
      (`self.ClientTouche` `Player Touche`))))

(event `ClientTouche`
  (params (`PLayer Touche` :type "/Game/Blueprint/BP_Eve Object Reference"))
  ;[1 0.1882 0.9528] Décrement vie
  ;;[1 1 1] affichage vie
  (`TextRenderComponent.K2_SetText` (`/Game/Blueprint/BP_Eve.txtVie` `PLayer Touche`) (`KismetTextLibrary.Conv_IntToText` (`/Game/Blueprint/BP_Eve.Vie` `PLayer Touche`))))

(event `ClientMort`
  (params (`PLayer Touche` :type "/Game/Blueprint/BP_Eve Object Reference"))
  ;[1 0.1882 0.9528] Décrement vie
  ;;[1 1 1] mort
  (`KismetSystemLibrary.Delay` 10.0)
  (set `/Game/Blueprint/BP_Eve.IsDead` false `PLayer Touche`)
  (set `/Game/Blueprint/BP_Eve.Vie` 100 `PLayer Touche`)
  (`self.ClientTouche` `PLayer Touche`))

(fn `UserConstructionScript`)