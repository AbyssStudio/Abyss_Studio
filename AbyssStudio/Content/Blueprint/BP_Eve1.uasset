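; BP_Eve1 is a player-controlled pawn with axis-driven movement and an on-screen crosshair.
; On BeginPlay it creates the HUD_Viseur widget, stores it as Scope and adds it to the viewport.
; MoveFront and MoveSide add movement along vectors from a yaw-only rotator, whose yaw is fed by the control rotation's roll rather than its yaw.
; LookSide adds controller yaw; no vertical look is handled here.
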(event `self.ReceiveBeginPlay`
  ;[0 1 0.8927] Viseur
  (bind _returnvalue (`|CreateWidget` "/Game/HUD/HUD_Viseur.HUD_Viseur_C"))
  (bind _output_get (set `self.Scope` _returnvalue))
  (`UserWidget.AddToViewport` _output_get 0))

(event `InputAxis|MoveFront`
  (params (AxisValue :type "Float (single-precision)"))
  ;[1 0.076 0] Déplacement
  ;;[1 0.3699 0.1586] Déplacement
  (`self.AddMovementInput` (`KismetMathLibrary.GetForwardVector` (`KismetMathLibrary.MakeRotator` 0.0 0.0 (.roll (`self.GetControlRotation`)))) AxisValue))

(event `InputAxis|MoveSide`
  (params (AxisValue :type "Float (single-precision)"))
  ;[1 0.076 0] Déplacement
  ;;[1 0.3699 0.1586] Déplacement
  (`self.AddMovementInput` (`KismetMathLibrary.GetRightVector` (`KismetMathLibrary.MakeRotator` 0.0 0.0 (.roll (`self.GetControlRotation`)))) AxisValue))

(event `InputAxis|LookSide`
  (params (AxisValue :type "Float (single-precision)"))
  ;[1 0.076 0] Déplacement
  ;;[1 0.5334 0] Gestion Caméra
  (`self.AddControllerYawInput` AxisValue))

(fn `UserConstructionScript`)